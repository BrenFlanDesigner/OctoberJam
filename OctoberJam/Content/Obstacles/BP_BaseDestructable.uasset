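; BP_BaseDestructable is a base destructible obstacle that handles damage from units with a tabletop-style armor save.
; AnyDamage ignores causers that are not BP_BaseUnitClass, then rolls a D6 reduced by the attacker's Piercing against Armor.
; A failed save subtracts the attacker's Damage variable from Health, ignoring the event's damage amount.
; Saves, hits and death only print messages; nothing destroys the actor.
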(event Game|Damage|EventAnyDamage
  (params (Damage :type Float%20%28single-precision%29) (DamageType :type Damage%20Type%20Object%20Reference) (InstigatedBy :type Controller%20Object%20Reference) (DamageCauser :type Actor%20Object%20Reference))
  (bind _asbp_base_unit_class (Utilities|Casting|CastToBP_BaseUnitClass DamageCauser))
  (bind _roll (CallFunction|D6))
  (if (>= (- _roll (Variables|/Game/Units/BP_BaseUnitClass.BP_BaseUnitClass_C|GetPiercing _asbp_base_unit_class)) (Variables|Default|GetArmor))
    (Development|PrintString "Armor Saved")
    (else
      (bind _output_get (Variables|Default|SetHealth (- (Variables|Default|GetHealth) (Variables|/Game/Units/BP_BaseUnitClass.BP_BaseUnitClass_C|GetDamage _asbp_base_unit_class))))
      (if (<= _output_get 0)
        (Development|PrintString "Dies")
        (else
          (Development|PrintString "took damage"))))))

(fn ConstructionScript)

(fn D6
  (return (Math|Random|RandomIntegerinRange 1 6)))