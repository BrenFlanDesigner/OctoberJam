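; Enemy spawner actor that periodically activates units from an enemy pool at random navigable points around itself.
; A looping timer started on BeginPlay calls SpawnEnemy, which proceeds only if a randomly picked pool entry is not already spawned.
; The pool is drawn again for the unit to spawn, so it can differ from the checked one.
; That unit spawns at a navmesh location within SpawnRadius, if one is found.
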(event Custom|SpawnEnemy
  (bind _enemypool (Variables|Default|GetEnemyPool))
  (bind _outitem (Utilities|Array|Random _enemypool))
  (if (not (Variables|/Game/Units/BP_BaseUnitClass.BP_BaseUnitClass_C|GetbIsSpawned _outitem))
    (Variables|Default|SetUnitToSpawn _outitem)
    (bind (_randomlocation _returnvalue) (Class|NavigationSystemV1|GetRandomLocationinNavigableRadius (Transformation|GetActorLocation) (Variables|Default|GetSpawnRadius) 0 0))
    (if _returnvalue
      (Default|Spawn (Variables|Default|GetUnitToSpawn) _randomlocation))))

(event EventBeginPlay
  (Utilities|Time|SetTimerbyFunctionName 0 "SpawnEnemy" 5.0 true))

(event Collision|EventActorBeginOverlap
  (params (OtherActor :type Actor%20Object%20Reference)))

(event EventTick
  (params (DeltaSeconds :type Float%20%28single-precision%29)))

(fn ConstructionScript)