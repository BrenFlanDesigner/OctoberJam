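; BP_Ability_Base is a base ability actor with a sphere hitbox and an aiming decal.
; The construction script sizes the sphere from HitboxSize and applies the AimingDecal material.
; AimAbility sets IsAiming and shows the decal, while StartAbility only hides it, leaving its TargetLocation input unused and IsAiming unchanged.
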(event EventBeginPlay)

(event Collision|EventActorBeginOverlap
  (params (OtherActor :type Actor%20Object%20Reference)))

(event EventTick
  (params (DeltaSeconds :type Float%20%28single-precision%29)))

(fn ConstructionScript
  (Components|Sphere|SetSphereRadius (Variables|Default|GetHitBox) (Variables|Default|GetHitboxSize) false)
  (Rendering|Components|Decal|SetDecalMaterial (Variables|Default|GetDecal) (Variables|Default|GetAimingDecal)))

(fn StartAbility
  (params (TargetLocation :type Vector))
  (Development|SetHiddeninGame (Variables|Default|GetDecal) true false))

(fn AimAbility
  (Variables|Default|SetbIsAiming true)
  (Development|SetHiddeninGame (Variables|Default|GetDecal) false false))