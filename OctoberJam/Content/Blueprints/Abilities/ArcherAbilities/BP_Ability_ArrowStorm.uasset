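; Archer Arrow Storm ability that rains five arrows on a target location, damaging enemy units.
; StartAbility moves the root there, randomizes arrow start points once within HitboxSize and loops RainArrows on a timer until AbilityDuration ends.
; Each cycle drops the arrows through staggered timelines, then runs a delayed damage pulse.
; The pulse loops over HitBox overlaps but always damages the first enemy, once per overlapping enemy.
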(event Custom|ArrowDamagePulse
  (bind _hitbox (Variables|Default|GetHitBox))
  (bind _overlappingactors (Collision|GetOverlappingActors _hitbox "/Game/Units/Enemies/BP_EnemyBaseUnit.BP_EnemyBaseUnit_C" :!class /Script/Engine.PrimitiveComponent))
  (bind _output (Utilities|Array|Get(acopy) _overlappingactors))
  (Utilities|IsValid _output
    (:Is%20Valid
      (for _array_element _overlappingactors
        (Game|Damage|ApplyDamage _output (Variables|Default|GetAbilityDamage) 0 (Variables|Default|GetOwningHero))))))

(event Custom|RainArrows
  (bind _arrowstart5 (Variables|Default|GetArrowStart5))
  (bind _arrowstart1 (Variables|Default|GetArrowStart1))
  (bind _arrowstart2 (Variables|Default|GetArrowStart2))
  (bind _arrowstart3 (Variables|Default|GetArrowStart3))
  (bind _arrowstart4 (Variables|Default|GetArrowStart4))
  (Utilities|FlowControl|Sequence
    (:then_0
      (bind _arrowdown (Timeline|ArrowMovement PlayFromStart)
        (:Update
          (Transformation|SetWorldLocation (Variables|Default|GetArrow1) (Math|Vector|Lerp(Vector) _arrowstart1 (- _arrowstart1 "0.000000,0.000000,1000.000000") _arrowdown) false false))))
    (:then_1
      (Utilities|FlowControl|Delay 0.1)
      (bind _arrowdown_2 (Timeline|Timeline PlayFromStart)
        (:Update
          (Transformation|SetWorldLocation (Variables|Default|GetArrow2) (Math|Vector|Lerp(Vector) _arrowstart2 (- _arrowstart2 "0.000000,0.000000,1000.000000") _arrowdown_2) false false))))
    (:then_2
      (Utilities|FlowControl|Delay 0.2)
      (bind _arrowdown_3 (Timeline|Timeline_0 PlayFromStart)
        (:Update
          (Transformation|SetWorldLocation (Variables|Default|GetArrow3) (Math|Vector|Lerp(Vector) _arrowstart3 (- _arrowstart3 "0.000000,0.000000,1000.000000") _arrowdown_3) false false))))
    (:then_3
      (Utilities|FlowControl|Delay 0.3)
      (bind _arrowdown_4 (Timeline|Timeline_1 PlayFromStart)
        (:Update
          (Transformation|SetWorldLocation (Variables|Default|GetArrow4) (Math|Vector|Lerp(Vector) _arrowstart4 (- _arrowstart4 "0.000000,0.000000,1000.000000") _arrowdown_4) false false))))
    (:then_4
      (Utilities|FlowControl|Delay 0.4)
      (bind _arrowdown_5 (Timeline|Timeline_2 PlayFromStart)
        (:Update
          (Transformation|SetWorldLocation (Variables|Default|GetArrow5) (Math|Vector|Lerp(Vector) _arrowstart5 (- _arrowstart5 "0.000000,0.000000,1000.000000") _arrowdown_5) false false))))
    (:then_5
      (Utilities|FlowControl|Delay 0.4)
      (CallFunction|ArrowDamagePulse))))

(event Custom|GenerateArrowStartLocations
  (bind _returnvalue (Transformation|GetActorLocation))
  (bind _hitboxsize (Variables|Default|GetHitboxSize))
  (bind _returnvalue_2 (* _hitboxsize -1.0))
  (bind _returnvalue_3 (* _hitboxsize -1.0))
  (bind _returnvalue_4 (Math|Random|RandomFloatinRange _returnvalue_2 _hitboxsize))
  (bind _returnvalue_5 (Math|Random|RandomFloatinRange _returnvalue_3 _hitboxsize))
  (bind _returnvalue_6 (+ _returnvalue (Math|Vector|MakeVector _returnvalue_5 _returnvalue_4 1e+03)))
  (Variables|Default|SetArrowStart1 _returnvalue_6)
  (Variables|Default|SetArrowStart2 _returnvalue_6)
  (Variables|Default|SetArrowStart3 _returnvalue_6)
  (Variables|Default|SetArrowStart4 _returnvalue_6)
  (Variables|Default|SetArrowStart5 _returnvalue_6)
  (Variables|Default|SetbIsReady false)
  (Utilities|FlowControl|Delay (Variables|Default|GetAbilityDuration))
  (Utilities|Time|ClearandInvalidateTimerbyHandle (Variables|Default|GetRainArrowsTimer))
  (Variables|Default|SetbIsReady true))

(event EventBeginPlay
  (|CallParentFunction) ; This node is disabled and will not be called.\nDrag off pins to build functionality.
)

(event Collision|EventActorBeginOverlap
  (params (OtherActor :type Actor%20Object%20Reference))
  (|CallParentFunction OtherActor) ; This node is disabled and will not be called.\nDrag off pins to build functionality.
)

(event EventTick
  (params (DeltaSeconds :type Float%20%28single-precision%29))
  (|CallParentFunction DeltaSeconds) ; This node is disabled and will not be called.\nDrag off pins to build functionality.
)

(fn ConstructionScript
  (|CallParentFunction))

(fn StartAbility
  (params (TargetLocation :type Vector :default "0, 0, 0"))
  (|CallParentFunction TargetLocation)
  (Transformation|SetWorldLocation (Variables|Default|GetDefaultSceneRoot) TargetLocation false true)
  (CallFunction|GenerateArrowStartLocations)
  (bind _returnvalue (Utilities|Time|SetTimerbyFunctionName 0 "RainArrows" 0.5 true))
  (Variables|Default|SetRainArrowsTimer _returnvalue))