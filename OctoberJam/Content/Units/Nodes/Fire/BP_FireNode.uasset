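; Fire node that ignites after a random delay, blocks pawns while burning, and can be extinguished by an interacting unit.
; FireLight shows the cone and progress-bar widget, then a looping Delay grows the fire toward full while nobody interacts.
; Interact runs its own Delay loop lowering that progress; at zero it hides the fire, unblocks pawns, releases the unit and schedules a random re-ignition.
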(event Custom|FireLight
  (bind _widgetref (Variables|Default|GetWidgetRef))
  ;[1 0.7343 0.4192] Light Fire
  (Rendering|SetVisibility (Variables|Default|GetCone) true false)
  (Collision|SetCollisionResponsetoChannel (Variables|Default|GetCapsuleComponent) "ECC_Pawn" "ECR_Block")
  (Variables|Default|SetbIsBurning true)
  (bind _output_get (Variables|Default|SetExtringuishProgress 0.6))
  (Default|Extinguish (Variables|Default|GetWidgetRef) _output_get)
  (Utilities|FlowControl|Delay 3.0 :!label _label)
  (if (Variables|Default|GetbIsBeingInteractedWith)
    (goto _label)
    (elif (Variables|Default|GetbIsBurning)
      (if (< (+ (Variables|Default|GetExtringuishProgress) 0.1) 1.0)
        (bind _output_get_2 (Variables|Default|SetExtringuishProgress (+ (Variables|Default|GetExtringuishProgress) 0.1)))
        (Default|Extinguish _widgetref _output_get_2)
        (goto _label)
        (else
          (bind _output_get_3 (Variables|Default|SetExtringuishProgress 1.0))
          (Default|Extinguish _widgetref _output_get_3)
          (goto _label))))))

(event EventBeginPlay
  ;[1 1 1] Set Timer for first ignite
  (|CallParentFunction)
  (bind _output_get (Variables|Default|SetIgniteTimer (Math|Random|RandomFloatinRange 5.0 6e+01)))
  (Utilities|Time|SetTimerbyEvent (delegate Custom|FireLight) _output_get)
  (Development|PrintString (Utilities|String|ToString(Float) _output_get) true true "(R=1.000000,G=0.072917,B=0.072917,A=1.000000)" (+ _output_get 3.0))
  (bind _aswbp_progress_bar (Utilities|Casting|CastToWBP_ProgressBar (UserInterface|GetWidget (Variables|Default|GetWidget))))
  (Variables|Default|SetWidgetRef _aswbp_progress_bar))

(event Collision|EventActorBeginOverlap
  (params (OtherActor :type Actor%20Object%20Reference)))

(event EventTick
  (params (DeltaSeconds :type Float%20%28single-precision%29)))

(event EventInteract
  (params (InteractingUnit :type BP%20Base%20Unit%20Class%20Object%20Reference))
  ;[0.5198 0.6751 1] Interact
  (Variables|Default|SetInteracting%20Unit InteractingUnit)
  (Variables|Default|SetbIsBeingInteractedWith true)
  ;;[1 1 1] Decriment the Extinguish progress
  (if (Variables|Default|GetbIsBeingInteractedWith) :!label _label
    (bind _output_get (Variables|Default|SetExtringuishProgress (- (Variables|Default|GetExtringuishProgress) 0.2)))
    (Utilities|FlowControl|Delay 1.2)
    (Default|Extinguish (Variables|Default|GetWidgetRef) _output_get)
    (if (<= _output_get 0.0)
      ;;[1 1 1] Extinguish fire if progressed enough, hide fire. Start Respawn timer
      (Variables|Default|SetbIsBeingInteractedWith false)
      (Variables|Default|SetbIsBurning false)
      (Rendering|SetVisibility (Variables|Default|GetCone) false false)
      (Collision|SetCollisionResponsetoChannel (Variables|Default|GetCapsuleComponent) "ECC_Pawn" "ECR_Ignore")
      (bind _output_get_2 (Variables|Default|SetIgniteTimer (Math|Random|RandomFloatinRange 15.0 45.0)))
      (Development|PrintString (Utilities|String|ToString(Float) _output_get_2))
      (Utilities|Time|SetTimerbyEvent (delegate Custom|FireLight) _output_get_2)
      (Default|InteractEnd (Variables|Default|GetInteracting%20Unit))
      (Variables|Default|SetbIsBeingInteractedWith false)
      (else
        (goto _label)))))

(event EventInteractEnd
  (Variables|Default|SetbIsBeingInteractedWith false))

(fn ConstructionScript
  (|CallParentFunction))

(fn GiveUnitReference
  (return self))