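; BP_HeroArcher is an archer hero unit with Arrow Storm as its only assigned ability.
; On BeginPlay, after the parent logic, it finds an existing BP_Ability_ArrowStorm actor in the world rather than spawning one.
; It sets itself as that actor's OwningHero and stores the actor as the sole entry in HeroAbilities.
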(event EventBeginPlay
  (|CallParentFunction)
  (bind _returnvalue (Actor|GetActorOfClass "/Game/Blueprints/Abilities/ArcherAbilities/BP_Ability_ArrowStorm.BP_Ability_ArrowStorm_C"))
  (Variables|/Game/Blueprints/Abilities/BP_Ability_Base.BP_Ability_Base_C|SetOwningHero _returnvalue self)
  (Variables|Default|SetHeroAbilities (Utilities|Array|MakeArray _returnvalue)))

(event Collision|EventActorBeginOverlap
  (params (OtherActor :type Actor%20Object%20Reference))
  (|CallParentFunction OtherActor) ; This node is disabled and will not be called.\nDrag off pins to build functionality.
)

(event EventTick
  (params (DeltaSeconds :type Float%20%28single-precision%29))
  (|CallParentFunction DeltaSeconds) ; This node is disabled and will not be called.\nDrag off pins to build functionality.
)

(fn ConstructionScript
  (|CallParentFunction))