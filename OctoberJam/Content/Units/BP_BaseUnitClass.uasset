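; Base class for team-tagged combat units, with selection highlight, spawn, movement, attack and death; IsBuilding disables movement and combat.
; A looping timer chases the target until in range, then attacks with a montage and delayed damage, rate-limited by a DoOnce.
; When the target is lost, a sphere trace seeks living opposing-tag units.
; Incoming damage faces a D6 armor-versus-piercing roll; DealDamage's accuracy and strength rolls are not called here.
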(event Custom|AttackEnemy
  ;[1 0.8597 0] Attack Event
  (if (not (Variables|Default|GetbIsBuilding))
    (Class|NavMovementComponent|StopActiveMovement (Variables|Character|GetCharacterMovement))
    (Animation|Montage|PlayMontage (Variables|Character|GetMesh) (Variables|Default|GetAttackMontage)
      (:then
        (Utilities|FlowControl|Delay 0.5)
        (Game|Damage|ApplyDamage (Variables|Default|GetTargetActor) (Math|Conversions|ToFloat(Integer) (Variables|Default|GetDamage)) 0 self)))))

(event Custom|CheckEnemyInRange
  ;[0 1 0.09229] Check if Target is in Range and initiate attack or Check for Aggro
  (if (not (Variables|Default|GetbIsBuilding))
    (bind _targetactor (Variables|Default|GetTargetActor)
      (:then
        (if (and (not (Variables|BP_BaseUnitClass_C|GetbIsDead _targetactor)) (not (Variables|Default|GetbIsDead)))
          (if (> (Transformation|GetDistanceTo _targetactor self) (Variables|Default|GetAttackRange))
            (CallFunction|MovetoActor (Variables|Default|GetTargetActor))
            (else
              (Utilities|FlowControl|DoOnce false
                (:Completed
                  (CallFunction|AttackEnemy)
                  (Utilities|FlowControl|Delay (Variables|Default|GetAttackRate))
                  (CallFunction|ResetAttackDoOnce)))))
          (else
            (Variables|Default|SetTargetActor 0)
            (Utilities|Time|ClearandInvalidateTimerbyHandle (Variables|Default|GetAttackTimer))
            (Utilities|FlowControl|Delay 0.2)
            (CallFunction|CheckforAgro))))
      (:else))))

(event Custom|Spawn
  (params (LocationToSpawn :type Vector))
  ;[0 0.03866 1] Spawning Events
  (Variables|Default|SetbIsSpawned true)
  (Transformation|SetActorLocation LocationToSpawn false true)
  (Variables|Default|SetbIsDead false)
  (Class|SkeletalMeshComponent|SetAnimClass (Variables|Character|GetMesh) (Utilities|GetClass (Variables|Default|GetAnimationInstance))))

(event Custom|Despawn
  ;[0 0.03866 1] Spawning Events
  (Variables|Default|SetbIsSpawned false))

(event Custom|CheckForAgro
  (bind _returnvalue (Transformation|GetActorLocation))
  ;[1 0 0.675] Check For Aggro
  (if (not (Variables|Default|GetbIsBuilding))
    (bind _outhits (Collision|MultiSphereTraceForObjects _returnvalue _returnvalue (Variables|Default|GetAggroRange) (Variables|Default|GetObject%20Types) false 0 "None"))
    (for _array_element _outhits
      (if (.bBlockingHit (Collision|BreakHitResult _array_element))
        (if (Actor|ActorHasTag (.HitActor (Collision|BreakHitResult _array_element)) (Variables|Default|GetTagToCheckFor))
          (bind _unit (Class|BPIActions|GiveUnitReference(Message) (.HitActor (Collision|BreakHitResult _array_element))))
          (if (not (Variables|BP_BaseUnitClass_C|GetbIsDead _unit))
            (Class|BPIActions|SetTargetActor(Message) self _unit)))))
    (Development|PrintString "AGRO CHECKED" true true "(R=1.000000,G=0.000000,B=0.006496,A=1.000000)" 4.0)))

(event Custom|ResetAttackDoOnce
  ;[0 1 0.09229] Check if Target is in Range and initiate attack or Check for Aggro
  (Utilities|FlowControl|DoOnce false) ; enters at Reset
)

(event EventBeginPlay
  (bind _mesh (Variables|Character|GetMesh))
  (bind _returnvalue (Components|SkeletalMesh|GetAnimInstance _mesh))
  ;[1 0 0.0285] BeginPlay, Determine Team and set Opposite Tag
  (Utilities|IsValid _returnvalue
    (:Is%20Valid
      (Variables|Default|SetAnimationInstance _returnvalue))
    (:Is%20Not%20Valid
      _))
  (if (Actor|ActorHasTag "FriendlyUnit")
    (Variables|Default|SetTagToCheckFor "EnemyUnit")
    (else
      (Variables|Default|SetTagToCheckFor "FriendlyUnit"))))

(event EventMovetoActor
  (params (TargetActor :type Actor%20Object%20Reference))
  ;[0 1 0.1088] Locomotion Events
  (if (not (Variables|Default|GetbIsBuilding))
    (AI|Navigation|SimpleMovetoActor (Pawn|GetController) TargetActor)))

(event EventMovetoLocation
  (params (LocationToMoveTo :type Vector :default "0, 0, 0"))
  ;[0 1 0.1088] Locomotion Events
  (if (not (Variables|Default|GetbIsBuilding))
    (AI|Navigation|SimpleMovetoLocation (Pawn|GetController) LocationToMoveTo)))

(event Game|Damage|EventAnyDamage
  (params (Damage :type Float%20%28single-precision%29) (DamageType :type Damage%20Type%20Object%20Reference) (InstigatedBy :type Controller%20Object%20Reference) (DamageCauser :type Actor%20Object%20Reference))
  ;[1 0 0.6724] Receive Damage Event
  (bind _asbp_base_unit_class (Utilities|Casting|CastToBP_BaseUnitClass DamageCauser))
  (CallFunction|TakeDamage (Variables|BP_BaseUnitClass_C|GetDamage _asbp_base_unit_class) (Variables|BP_BaseUnitClass_C|GetPiercing _asbp_base_unit_class)))

(event EventSetTargetActor
  (params (NewTargetActor :type BP%20Base%20Unit%20Class%20Object%20Reference))
  ;[0 0.5509 1] Set Target actor with a Base unit Object Reference
  (if (not (Variables|Default|GetbIsBuilding))
    (Variables|Default|SetTargetActor NewTargetActor)
    (bind _returnvalue (Utilities|Time|SetTimerbyFunctionName 0 "CheckEnemyInRange" 0.1 true))
    (Variables|Default|SetAttackTimer _returnvalue)
    (CallFunction|CheckEnemyinRange)))

(event EventSelectUnit
  ;[1 1 1] Selected Highlight
  (Development|SetHiddeninGame (Variables|Default|GetHighlight) false false))

(event EventDeselect
  ;[1 1 1] Selected Highlight
  (Development|SetHiddeninGame (Variables|Default|GetHighlight) true false))

(fn ConstructionScript
  (Rendering|Material|SetMaterial (Variables|Default|GetHighlight) 0 (Variables|Default|GetHighlightMaterial)))

(fn TakeDamage
  (params (IncomingDamage :type Integer) (Incoming%20Pierce :type Integer))
  (bind _value (CallFunction|D6))
  (if (>= _value (- (Variables|Default|GetArmor) Incoming%20Pierce))
    (Development|PrintString "Armor Saved damage")
    (else
      (Components|Animation|PlayAnimation (Variables|Character|GetMesh) (Variables|Default|GetHitAnimation) false)
      (bind _output_get (Variables|Default|SetCurHealth (- (Variables|Default|GetCurHealth) IncomingDamage)))
      (if (<= _output_get 0)
        (CallFunction|Death)))))

(fn D6
  (return (Math|Random|RandomIntegerinRange 1 6)))

(fn Death
  (Variables|Default|SetbIsDead true)
  (Components|Animation|PlayAnimation (Variables|Character|GetMesh) (Variables|Default|GetDieAnimation) false))

(fn DealDamage
  (params (EnemyTarget :type Actor%20Object%20Reference))
  (bind _value (CallFunction|D6))
  (if (>= _value (Variables|Default|GetAccuracy))
    (bind _value_2 (CallFunction|D6))
    (if (>= _value_2 (Variables|Default|GetStrength))
      (Game|Damage|ApplyDamage EnemyTarget (Math|Conversions|ToFloat(Integer) (Variables|Default|GetDamage)) 0 self)
      (else
        (Development|PrintString "Attack not strong enough")))
    (else
      (Development|PrintString "Attack Misses"))))

(fn GiveUnitReference
  (return self))