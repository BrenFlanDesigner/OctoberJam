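; Enemy rally point that the player captures by holding its sphere with at least three friendly units and no enemies.
; Tag-checked overlaps count units per side, and a looping one-second timer drains capture progress while held, otherwise restores it toward maximum.
; The timer also pushes the percentage to a widget.
; On capture it hides the mesh, stops the timer and sends InteractMessage to each spawner in SpawnersToDeactivate.
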(event OnComponentBeginOverlap(CapturePoint)
  (params (OverlappedComponent :type Primitive%20Component%20Object%20Reference) (OtherActor :type Actor%20Object%20Reference) (OtherComp :type Primitive%20Component%20Object%20Reference) (OtherBodyIndex :type Integer) (bFromSweep :type Boolean) (SweepResult :type Hit%20Result%20Structure%20%28by%20ref%29))
  (if (Actor|ActorHasTag OtherActor "FriendlyUnit")
    (Math|Integer|IncrementInt (Variables|Default|GetPlayerUnits)
      (:%20%20
        (Development|PrintString "PLAYER IN" true true "(R=1.000000,G=0.000000,B=0.800881,A=1.000000)" 3.0)))
    (elif (Actor|ActorHasTag OtherActor "EnemyUnit")
      (Math|Integer|IncrementInt (Variables|Default|GetEnemyUnits)
        (:%20%20
          (Development|PrintString "ENEMY IN" true true "(R=1.000000,G=0.000000,B=0.800881,A=1.000000)" 3.0))))))

(event OnComponentEndOverlap(CapturePoint)
  (params (OverlappedComponent :type Primitive%20Component%20Object%20Reference) (OtherActor :type Actor%20Object%20Reference) (OtherComp :type Primitive%20Component%20Object%20Reference) (OtherBodyIndex :type Integer))
  (if (Actor|ActorHasTag OtherActor "FriendlyUnit")
    (Math|Integer|DecrementInt (Variables|Default|GetPlayerUnits)
      (:%20%20
        (Development|PrintString "PLAYER OUT" true true "(R=1.000000,G=0.000000,B=0.800881,A=1.000000)" 3.0)))
    (elif (Actor|ActorHasTag OtherActor "EnemyUnit")
      (Math|Integer|DecrementInt (Variables|Default|GetEnemyUnits)
        (:%20%20
          (Development|PrintString "ENEMY OUT" true true "(R=1.000000,G=0.000000,B=0.054821,A=1.000000)" 3.0))))))

(event Custom|CheckCapStatus
  (if (and (== (Variables|Default|GetEnemyUnits) 0) (>= (Variables|Default|GetPlayerUnits) 3))
    (if (<= (- (Variables|Default|GetCurrentCapture) (Variables|Default|GetCapInterval)) 0.0)
      (Variables|Default|SetbIsCapped true)
      (Development|SetHiddeninGame (Variables|Default|GetSkeletalMesh) true true)
      (else
        (Variables|Default|SetCurrentCapture (- (Variables|Default|GetCurrentCapture) (Variables|Default|GetCapInterval)))))
    (elif (>= (+ (Variables|Default|GetCurrentCapture) (Variables|Default|GetCapInterval)) (Variables|Default|GetMaxCapture))
      (Variables|Default|SetCurrentCapture (Variables|Default|GetMaxCapture))
      (else
        (Variables|Default|SetCurrentCapture (+ (Variables|Default|GetCurrentCapture) (Variables|Default|GetCapInterval))))))
  (Class|BPIActions|SendPercent(Message) (UserInterface|GetWidget (Variables|Default|GetWidget)) (/ (Variables|Default|GetCurrentCapture) (Variables|Default|GetMaxCapture)))
  (if (Variables|Default|GetbIsCapped)
    (Utilities|Time|ClearandInvalidateTimerbyHandle (Variables|Default|GetCapStatusTimer))
    (for _array_element (Variables|Default|GetSpawnersToDeactivate)
      (Class|BPIActions|Interact(Message) _array_element))))

(event EventBeginPlay
  (bind _returnvalue (Utilities|Time|SetTimerbyFunctionName 0 "CheckCapStatus" 1.0 true))
  (Variables|Default|SetCapStatusTimer _returnvalue)
  (Class|BPIActions|SendPercent(Message) (UserInterface|GetWidget (Variables|Default|GetWidget)) (/ (Variables|Default|GetCurrentCapture) (Variables|Default|GetMaxCapture))))

(fn ConstructionScript
  (Components|Sphere|SetSphereRadius (Variables|Default|GetCapturePoint) (Variables|Default|GetCaptureRadius) true))